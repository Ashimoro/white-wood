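; Level intro dialogue actor that plays a timed monologue chosen by the pigeon player's day and timeline value.
; On BeginPlay it switches on BP_Pigeon's DayIntVariable into branches for Day 1 and the truth/false timelines of Days 2 and 3.
; Each branch chains hard-coded DataTable row lookups and Delays to update one UiTest widget, then sets Enddialogue and hides it.
; Day 5 and unmatched values create the widget but hide it immediately.
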(event EventBeginPlay
  (bind _asbp_pigeon (Utilities|Casting|CastToBP_Pigeon (Game|Player|GetPlayerPawn 0))
    (:then
      (switch int (Variables|/Game/_TopDown/Blueprints/BP_Pigeon.BP_Pigeon_C|GetDayIntVariable _asbp_pigeon)
        (:Default
          ;[0.15 0.15 0.15 0.5] dialoge line 46
          (bind _returnvalue (Utilities|GetDataTableRow (Variables|Default|GetData%20Table) "55" :!label _label)
            (:then
              (bind _returnvalue_2 (UserInterface|CreateWidget "/Game/_Dialogue/UiTest.UiTest_C" 0 (Utilities|Text|ToText(Name) (Variables|Default|GetSpeakerName)) (.IntroDialogue (Utilities|Struct|Breakdialogue_Structure _returnvalue))))
              (bind _output_get (Variables|Default|SetdialogueWidget _returnvalue_2))
              (UserInterface|Viewport|AddtoViewport _output_get 0)
              (Variables|Default|SetRow%20Name (.Row (Utilities|Struct|Breakdialogue_Structure _returnvalue)))
              (Variables|Default|SetData%20Table (.Datatable (Utilities|Struct|Breakdialogue_Structure _returnvalue)))
              (Variables|Default|Setenddialogue (.EndDialogue (Utilities|Struct|Breakdialogue_Structure _returnvalue)))
              (Widget|SetVisibility (Variables|Default|GetdialogueWidget) "Hidden"))))
        (:0
          (Development|PrintString "Dialogue Branch: Day 1")
          ;[0.15 0.15 0.15 0.5] dialoge line 1
          (bind _returnvalue_3 (Utilities|GetDataTableRow (Variables|Default|GetData%20Table) (Variables|Default|GetRow%20Name))
            (:then
              (bind _returnvalue_4 (UserInterface|CreateWidget "/Game/_Dialogue/UiTest.UiTest_C" 0 (Utilities|Text|ToText(Name) (Variables|Default|GetSpeakerName)) (.IntroDialogue (Utilities|Struct|Breakdialogue_Structure _returnvalue_3))))
              (bind _output_get_2 (Variables|Default|SetdialogueWidget _returnvalue_4))
              (UserInterface|Viewport|AddtoViewport _output_get_2 0)
              (Variables|Default|SetRow%20Name (.Row (Utilities|Struct|Breakdialogue_Structure _returnvalue_3)))
              (Variables|Default|SetData%20Table (.Datatable (Utilities|Struct|Breakdialogue_Structure _returnvalue_3)))
              (Variables|Default|Setenddialogue (.EndDialogue (Utilities|Struct|Breakdialogue_Structure _returnvalue_3)))
              (Utilities|FlowControl|Delay 5.0)
              ;[0.15 0.15 0.15 0.5] dialogue line 2
              (bind _returnvalue_5 (Utilities|GetDataTableRow (Variables|Default|GetData%20Table) "2")
                (:then
                  (Default|UpdateDialogueTest (Variables|Default|GetdialogueWidget) (.IntroDialogue (Utilities|Struct|Breakdialogue_Structure _returnvalue_5)))
                  (Variables|Default|SetRow%20Name (.Row (Utilities|Struct|Breakdialogue_Structure _returnvalue_5)))
                  (Variables|Default|SetData%20Table (.Datatable (Utilities|Struct|Breakdialogue_Structure _returnvalue_5)))
                  (Utilities|FlowControl|Delay 5.0)
                  ;[0.15 0.15 0.15 0.5] dialogue line 3
                  (bind _returnvalue_6 (Utilities|GetDataTableRow (Variables|Default|GetData%20Table) "3")
                    (:then
                      (Default|UpdateDialogueTest (Variables|Default|GetdialogueWidget) (.IntroDialogue (Utilities|Struct|Breakdialogue_Structure _returnvalue_6)))
                      (Variables|Default|SetRow%20Name (.Row (Utilities|Struct|Breakdialogue_Structure _returnvalue_6)))
                      (Variables|Default|SetData%20Table (.Datatable (Utilities|Struct|Breakdialogue_Structure _returnvalue_6)))
                      (Utilities|FlowControl|Delay 5.0)
                      ;[0.15 0.15 0.15 0.5] dialogue line 4
                      (bind _returnvalue_7 (Utilities|GetDataTableRow (Variables|Default|GetData%20Table) "4")
                        (:then
                          (Default|UpdateDialogueTest (Variables|Default|GetdialogueWidget) (.IntroDialogue (Utilities|Struct|Breakdialogue_Structure _returnvalue_7)))
                          (Variables|Default|SetRow%20Name (.Row (Utilities|Struct|Breakdialogue_Structure _returnvalue_7)))
                          (Utilities|FlowControl|Delay 5.0)
                          ;[0.15 0.15 0.15 0.5] dialogue line 5
                          (bind _returnvalue_8 (Utilities|GetDataTableRow (Variables|Default|GetData%20Table) "5")
                            (:then
                              (Default|UpdateDialogueTest (Variables|Default|GetdialogueWidget) (.IntroDialogue (Utilities|Struct|Breakdialogue_Structure _returnvalue_8)))
                              (Variables|Default|SetRow%20Name (.Row (Utilities|Struct|Breakdialogue_Structure _returnvalue_8)))
                              (Utilities|FlowControl|Delay 5.0)
                              ;[0.15 0.15 0.15 0.5] dialogue line 6
                              (bind _returnvalue_9 (Utilities|GetDataTableRow (Variables|Default|GetData%20Table) "6")
                                (:then
                                  (Default|UpdateDialogueTest (Variables|Default|GetdialogueWidget) (.IntroDialogue (Utilities|Struct|Breakdialogue_Structure _returnvalue_9)))
                                  (Variables|Default|SetRow%20Name (.Row (Utilities|Struct|Breakdialogue_Structure _returnvalue_9)))
                                  (Utilities|FlowControl|Delay 5.0)
                                  ;[0.15 0.15 0.15 0.5] dialogue line 7
                                  (bind _returnvalue_10 (Utilities|GetDataTableRow (Variables|Default|GetData%20Table) "7")
                                    (:then
                                      (Default|UpdateDialogueTest (Variables|Default|GetdialogueWidget) (.IntroDialogue (Utilities|Struct|Breakdialogue_Structure _returnvalue_10)))
                                      (Variables|Default|SetRow%20Name (.Row (Utilities|Struct|Breakdialogue_Structure _returnvalue_10)))
                                      (Utilities|FlowControl|Delay 5.0)
                                      ;[0.15 0.15 0.15 0.5] dialogue line 8
                                      (bind _returnvalue_11 (Utilities|GetDataTableRow (Variables|Default|GetData%20Table) "8")
                                        (:then
                                          (Default|UpdateDialogueTest (Variables|Default|GetdialogueWidget) (.IntroDialogue (Utilities|Struct|Breakdialogue_Structure _returnvalue_11)))
                                          (Variables|Default|SetRow%20Name (.Row (Utilities|Struct|Breakdialogue_Structure _returnvalue_11)))
                                          (Utilities|FlowControl|Delay 5.0)
                                          ;[0.15 0.15 0.15 0.5] dialogue line 9
                                          (bind _returnvalue_12 (Utilities|GetDataTableRow (Variables|Default|GetData%20Table) "9")
                                            (:then
                                              (Default|UpdateDialogueTest (Variables|Default|GetdialogueWidget) (.IntroDialogue (Utilities|Struct|Breakdialogue_Structure _returnvalue_12)))
                                              (Variables|Default|SetRow%20Name (.Row (Utilities|Struct|Breakdialogue_Structure _returnvalue_12)))
                                              (Utilities|FlowControl|Delay 5.0)
                                              ;[0.15 0.15 0.15 0.5] dialogue line 10
                                              (bind _returnvalue_13 (Utilities|GetDataTableRow (Variables|Default|GetData%20Table) "10")
                                                (:then
                                                  (Default|UpdateDialogueTest (Variables|Default|GetdialogueWidget) (.IntroDialogue (Utilities|Struct|Breakdialogue_Structure _returnvalue_13)))
                                                  (Variables|Default|SetRow%20Name (.Row (Utilities|Struct|Breakdialogue_Structure _returnvalue_13)))
                                                  (Utilities|FlowControl|Delay 5.0)
                                                  ;[0.15 0.15 0.15 0.5] dialogue line 11
                                                  (bind _returnvalue_14 (Utilities|GetDataTableRow (Variables|Default|GetData%20Table) "11")
                                                    (:then
                                                      (Default|UpdateDialogueTest (Variables|Default|GetdialogueWidget) (.IntroDialogue (Utilities|Struct|Breakdialogue_Structure _returnvalue_14)))
                                                      (Variables|Default|SetRow%20Name (.Row (Utilities|Struct|Breakdialogue_Structure _returnvalue_14)))
                                                      (Utilities|FlowControl|Delay 5.0)
                                                      ;[0.15 0.15 0.15 0.5] dialogue line 12
                                                      (bind _returnvalue_15 (Utilities|GetDataTableRow (Variables|Default|GetData%20Table) "12")
                                                        (:then
                                                          (Default|UpdateDialogueTest (Variables|Default|GetdialogueWidget) (.IntroDialogue (Utilities|Struct|Breakdialogue_Structure _returnvalue_15)))
                                                          (Variables|Default|SetRow%20Name (.Row (Utilities|Struct|Breakdialogue_Structure _returnvalue_15)))
                                                          ;[0.15 0.15 0.15 0.5] hide intro dialogue
                                                          (Variables|Default|Setenddialogue true)
                                                          (Utilities|FlowControl|Delay 5.0)
                                                          (Widget|SetVisibility (Variables|Default|GetdialogueWidget) "Hidden"))))))))))))))))))))))))))
        (:1
          (Development|PrintString "Dialogue Branch: Day 2 TRUTH Timeline")
          ;[0.15 0.15 0.15 0.5] dialoge line 1
          (bind _returnvalue_16 (Utilities|GetDataTableRow (Variables|Default|GetData%20Table) "16")
            (:then
              (bind _returnvalue_17 (UserInterface|CreateWidget "/Game/_Dialogue/UiTest.UiTest_C" 0 (Utilities|Text|ToText(Name) (Variables|Default|GetSpeakerName)) (.IntroDialogue (Utilities|Struct|Breakdialogue_Structure _returnvalue_16))))
              (bind _output_get_3 (Variables|Default|SetdialogueWidget _returnvalue_17))
              (UserInterface|Viewport|AddtoViewport _output_get_3 0)
              (Variables|Default|SetRow%20Name (.Row (Utilities|Struct|Breakdialogue_Structure _returnvalue_16)))
              (Variables|Default|SetData%20Table (.Datatable (Utilities|Struct|Breakdialogue_Structure _returnvalue_16)))
              (Variables|Default|Setenddialogue (.EndDialogue (Utilities|Struct|Breakdialogue_Structure _returnvalue_16)))
              (Utilities|FlowControl|Delay 5.0)
              ;[0.15 0.15 0.15 0.5] dialogue line 2
              (bind _returnvalue_18 (Utilities|GetDataTableRow (Variables|Default|GetData%20Table) "17")
                (:then
                  (Default|UpdateDialogueTest (Variables|Default|GetdialogueWidget) (.IntroDialogue (Utilities|Struct|Breakdialogue_Structure _returnvalue_18)))
                  (Variables|Default|SetRow%20Name (.Row (Utilities|Struct|Breakdialogue_Structure _returnvalue_18)))
                  (Variables|Default|SetData%20Table (.Datatable (Utilities|Struct|Breakdialogue_Structure _returnvalue_18)))
                  (Utilities|FlowControl|Delay 5.0)
                  ;[0.15 0.15 0.15 0.5] dialogue line 2
                  (bind _returnvalue_19 (Utilities|GetDataTableRow (Variables|Default|GetData%20Table) "18")
                    (:then
                      (Default|UpdateDialogueTest (Variables|Default|GetdialogueWidget) (.IntroDialogue (Utilities|Struct|Breakdialogue_Structure _returnvalue_19)))
                      (Variables|Default|SetRow%20Name (.Row (Utilities|Struct|Breakdialogue_Structure _returnvalue_19)))
                      (Variables|Default|SetData%20Table (.Datatable (Utilities|Struct|Breakdialogue_Structure _returnvalue_19)))
                      (Utilities|FlowControl|Delay 5.0)
                      ;[0.15 0.15 0.15 0.5] dialogue line 2
                      (bind _returnvalue_20 (Utilities|GetDataTableRow (Variables|Default|GetData%20Table) "19")
                        (:then
                          (Default|UpdateDialogueTest (Variables|Default|GetdialogueWidget) (.IntroDialogue (Utilities|Struct|Breakdialogue_Structure _returnvalue_20)))
                          (Variables|Default|SetRow%20Name (.Row (Utilities|Struct|Breakdialogue_Structure _returnvalue_20)))
                          (Variables|Default|SetData%20Table (.Datatable (Utilities|Struct|Breakdialogue_Structure _returnvalue_20)))
                          (Utilities|FlowControl|Delay 5.0)
                          ;[0.15 0.15 0.15 0.5] dialogue line 2
                          (bind _returnvalue_21 (Utilities|GetDataTableRow (Variables|Default|GetData%20Table) "20")
                            (:then
                              (Default|UpdateDialogueTest (Variables|Default|GetdialogueWidget) (.IntroDialogue (Utilities|Struct|Breakdialogue_Structure _returnvalue_21)))
                              (Variables|Default|SetRow%20Name (.Row (Utilities|Struct|Breakdialogue_Structure _returnvalue_21)))
                              (Variables|Default|SetData%20Table (.Datatable (Utilities|Struct|Breakdialogue_Structure _returnvalue_21)))
                              (Utilities|FlowControl|Delay 5.0)
                              ;[0.15 0.15 0.15 0.5] dialogue line 21
                              (bind _returnvalue_22 (Utilities|GetDataTableRow (Variables|Default|GetData%20Table) "21")
                                (:then
                                  (Default|UpdateDialogueTest (Variables|Default|GetdialogueWidget) (.IntroDialogue (Utilities|Struct|Breakdialogue_Structure _returnvalue_22)))
                                  (Variables|Default|SetRow%20Name (.Row (Utilities|Struct|Breakdialogue_Structure _returnvalue_22)))
                                  (Variables|Default|SetData%20Table (.Datatable (Utilities|Struct|Breakdialogue_Structure _returnvalue_22)))
                                  (Utilities|FlowControl|Delay 5.0)
                                  ;[0.15 0.15 0.15 0.5] dialogue line 22
                                  (bind _returnvalue_23 (Utilities|GetDataTableRow (Variables|Default|GetData%20Table) "22")
                                    (:then
                                      (Default|UpdateDialogueTest (Variables|Default|GetdialogueWidget) (.IntroDialogue (Utilities|Struct|Breakdialogue_Structure _returnvalue_23)))
                                      (Variables|Default|SetRow%20Name (.Row (Utilities|Struct|Breakdialogue_Structure _returnvalue_23)))
                                      (Variables|Default|SetData%20Table (.Datatable (Utilities|Struct|Breakdialogue_Structure _returnvalue_23)))
                                      (Utilities|FlowControl|Delay 5.0)
                                      ;[0.15 0.15 0.15 0.5] dialogue line 23
                                      (bind _returnvalue_24 (Utilities|GetDataTableRow (Variables|Default|GetData%20Table) "23")
                                        (:then
                                          (Default|UpdateDialogueTest (Variables|Default|GetdialogueWidget) (.IntroDialogue (Utilities|Struct|Breakdialogue_Structure _returnvalue_24)))
                                          (Variables|Default|SetRow%20Name (.Row (Utilities|Struct|Breakdialogue_Structure _returnvalue_24)))
                                          (Variables|Default|SetData%20Table (.Datatable (Utilities|Struct|Breakdialogue_Structure _returnvalue_24)))
                                          (Utilities|FlowControl|Delay 5.0)
                                          ;[0.15 0.15 0.15 0.5] dialogue line 24
                                          (bind _returnvalue_25 (Utilities|GetDataTableRow (Variables|Default|GetData%20Table) "24")
                                            (:then
                                              (Default|UpdateDialogueTest (Variables|Default|GetdialogueWidget) (.IntroDialogue (Utilities|Struct|Breakdialogue_Structure _returnvalue_25)))
                                              (Variables|Default|SetRow%20Name (.Row (Utilities|Struct|Breakdialogue_Structure _returnvalue_25)))
                                              (Variables|Default|SetData%20Table (.Datatable (Utilities|Struct|Breakdialogue_Structure _returnvalue_25)))
                                              (Utilities|FlowControl|Delay 5.0)
                                              ;[0.15 0.15 0.15 0.5] dialogue line 25
                                              (bind _returnvalue_26 (Utilities|GetDataTableRow (Variables|Default|GetData%20Table) "25")
                                                (:then
                                                  (Default|UpdateDialogueTest (Variables|Default|GetdialogueWidget) (.IntroDialogue (Utilities|Struct|Breakdialogue_Structure _returnvalue_26)))
                                                  (Variables|Default|SetRow%20Name (.Row (Utilities|Struct|Breakdialogue_Structure _returnvalue_26)))
                                                  (Variables|Default|SetData%20Table (.Datatable (Utilities|Struct|Breakdialogue_Structure _returnvalue_26)))
                                                  (Utilities|FlowControl|Delay 4.0)
                                                  ;[0.15 0.15 0.15 0.5] dialogue line 26
                                                  (bind _returnvalue_27 (Utilities|GetDataTableRow (Variables|Default|GetData%20Table) "26")
                                                    (:then
                                                      (Default|UpdateDialogueTest (Variables|Default|GetdialogueWidget) (.IntroDialogue (Utilities|Struct|Breakdialogue_Structure _returnvalue_27)))
                                                      (Variables|Default|SetRow%20Name (.Row (Utilities|Struct|Breakdialogue_Structure _returnvalue_27)))
                                                      (Variables|Default|SetData%20Table (.Datatable (Utilities|Struct|Breakdialogue_Structure _returnvalue_27)))
                                                      (Utilities|FlowControl|Delay 5.0)
                                                      ;[0.15 0.15 0.15 0.5] dialogue line 27 - END
                                                      (bind _returnvalue_28 (Utilities|GetDataTableRow (Variables|Default|GetData%20Table) "27")
                                                        (:then
                                                          (Default|UpdateDialogueTest (Variables|Default|GetdialogueWidget) (.IntroDialogue (Utilities|Struct|Breakdialogue_Structure _returnvalue_28)))
                                                          (Variables|Default|SetRow%20Name (.Row (Utilities|Struct|Breakdialogue_Structure _returnvalue_28)))
                                                          (Variables|Default|SetData%20Table (.Datatable (Utilities|Struct|Breakdialogue_Structure _returnvalue_28)))
                                                          ;[0.15 0.15 0.15 0.5] hide intro dialogue
                                                          (Variables|Default|Setenddialogue true)
                                                          (Utilities|FlowControl|Delay 5.0)
                                                          (Widget|SetVisibility (Variables|Default|GetdialogueWidget) "Hidden"))))))))))))))))))))))))))
        (:2
          (Development|PrintString "Dialogue Branch: Day 2 FALSE Timeline")
          ;[0.15 0.15 0.15 0.5] dialoge line 28
          (bind _returnvalue_29 (Utilities|GetDataTableRow (Variables|Default|GetData%20Table) "28")
            (:then
              (bind _returnvalue_30 (UserInterface|CreateWidget "/Game/_Dialogue/UiTest.UiTest_C" 0 (Utilities|Text|ToText(Name) (Variables|Default|GetSpeakerName)) (.IntroDialogue (Utilities|Struct|Breakdialogue_Structure _returnvalue_29))))
              (bind _output_get_4 (Variables|Default|SetdialogueWidget _returnvalue_30))
              (UserInterface|Viewport|AddtoViewport _output_get_4 0)
              (Variables|Default|SetRow%20Name (.Row (Utilities|Struct|Breakdialogue_Structure _returnvalue_29)))
              (Variables|Default|SetData%20Table (.Datatable (Utilities|Struct|Breakdialogue_Structure _returnvalue_29)))
              (Variables|Default|Setenddialogue (.EndDialogue (Utilities|Struct|Breakdialogue_Structure _returnvalue_29)))
              (Utilities|FlowControl|Delay 5.0)
              ;[0.15 0.15 0.15 0.5] dialogue line 29
              (bind _returnvalue_31 (Utilities|GetDataTableRow (Variables|Default|GetData%20Table) "29")
                (:then
                  (Default|UpdateDialogueTest (Variables|Default|GetdialogueWidget) (.IntroDialogue (Utilities|Struct|Breakdialogue_Structure _returnvalue_31)))
                  (Variables|Default|SetRow%20Name (.Row (Utilities|Struct|Breakdialogue_Structure _returnvalue_31)))
                  (Variables|Default|SetData%20Table (.Datatable (Utilities|Struct|Breakdialogue_Structure _returnvalue_31)))
                  (Utilities|FlowControl|Delay 5.0)
                  ;[0.15 0.15 0.15 0.5] dialogue line 30
                  (bind _returnvalue_32 (Utilities|GetDataTableRow (Variables|Default|GetData%20Table) "30")
                    (:then
                      (Default|UpdateDialogueTest (Variables|Default|GetdialogueWidget) (.IntroDialogue (Utilities|Struct|Breakdialogue_Structure _returnvalue_32)))
                      (Variables|Default|SetRow%20Name (.Row (Utilities|Struct|Breakdialogue_Structure _returnvalue_32)))
                      (Variables|Default|SetData%20Table (.Datatable (Utilities|Struct|Breakdialogue_Structure _returnvalue_32)))
                      (Utilities|FlowControl|Delay 5.0)
                      ;[0.15 0.15 0.15 0.5] dialogue line 31
                      (bind _returnvalue_33 (Utilities|GetDataTableRow (Variables|Default|GetData%20Table) "31")
                        (:then
                          (Default|UpdateDialogueTest (Variables|Default|GetdialogueWidget) (.IntroDialogue (Utilities|Struct|Breakdialogue_Structure _returnvalue_33)))
                          (Variables|Default|SetRow%20Name (.Row (Utilities|Struct|Breakdialogue_Structure _returnvalue_33)))
                          (Variables|Default|SetData%20Table (.Datatable (Utilities|Struct|Breakdialogue_Structure _returnvalue_33)))
                          (Utilities|FlowControl|Delay 5.0)
                          ;[0.15 0.15 0.15 0.5] dialogue line 32
                          (bind _returnvalue_34 (Utilities|GetDataTableRow (Variables|Default|GetData%20Table) "32")
                            (:then
                              (Default|UpdateDialogueTest (Variables|Default|GetdialogueWidget) (.IntroDialogue (Utilities|Struct|Breakdialogue_Structure _returnvalue_34)))
                              (Variables|Default|SetRow%20Name (.Row (Utilities|Struct|Breakdialogue_Structure _returnvalue_34)))
                              (Variables|Default|SetData%20Table (.Datatable (Utilities|Struct|Breakdialogue_Structure _returnvalue_34)))
                              (Utilities|FlowControl|Delay 5.0)
                              ;[0.15 0.15 0.15 0.5] dialogue line 33
                              (bind _returnvalue_35 (Utilities|GetDataTableRow (Variables|Default|GetData%20Table) "33")
                                (:then
                                  (Default|UpdateDialogueTest (Variables|Default|GetdialogueWidget) (.IntroDialogue (Utilities|Struct|Breakdialogue_Structure _returnvalue_35)))
                                  (Variables|Default|SetRow%20Name (.Row (Utilities|Struct|Breakdialogue_Structure _returnvalue_35)))
                                  (Variables|Default|SetData%20Table (.Datatable (Utilities|Struct|Breakdialogue_Structure _returnvalue_35)))
                                  (Utilities|FlowControl|Delay 5.0)
                                  ;[0.15 0.15 0.15 0.5] dialogue line 34
                                  (bind _returnvalue_36 (Utilities|GetDataTableRow (Variables|Default|GetData%20Table) "34")
                                    (:then
                                      (Default|UpdateDialogueTest (Variables|Default|GetdialogueWidget) (.IntroDialogue (Utilities|Struct|Breakdialogue_Structure _returnvalue_36)))
                                      (Variables|Default|SetRow%20Name (.Row (Utilities|Struct|Breakdialogue_Structure _returnvalue_36)))
                                      (Variables|Default|SetData%20Table (.Datatable (Utilities|Struct|Breakdialogue_Structure _returnvalue_36)))
                                      (Utilities|FlowControl|Delay 5.0)
                                      ;[0.15 0.15 0.15 0.5] dialogue line 35
                                      (bind _returnvalue_37 (Utilities|GetDataTableRow (Variables|Default|GetData%20Table) "35")
                                        (:then
                                          (Default|UpdateDialogueTest (Variables|Default|GetdialogueWidget) (.IntroDialogue (Utilities|Struct|Breakdialogue_Structure _returnvalue_37)))
                                          (Variables|Default|SetRow%20Name (.Row (Utilities|Struct|Breakdialogue_Structure _returnvalue_37)))
                                          (Variables|Default|SetData%20Table (.Datatable (Utilities|Struct|Breakdialogue_Structure _returnvalue_37)))
                                          (Utilities|FlowControl|Delay 5.0)
                                          ;[0.15 0.15 0.15 0.5] dialogue line 36
                                          (bind _returnvalue_38 (Utilities|GetDataTableRow (Variables|Default|GetData%20Table) "36")
                                            (:then
                                              (Default|UpdateDialogueTest (Variables|Default|GetdialogueWidget) (.IntroDialogue (Utilities|Struct|Breakdialogue_Structure _returnvalue_38)))
                                              (Variables|Default|SetRow%20Name (.Row (Utilities|Struct|Breakdialogue_Structure _returnvalue_38)))
                                              (Variables|Default|SetData%20Table (.Datatable (Utilities|Struct|Breakdialogue_Structure _returnvalue_38)))
                                              (Utilities|FlowControl|Delay 5.0)
                                              ;[0.15 0.15 0.15 0.5] dialogue line 37
                                              (bind _returnvalue_39 (Utilities|GetDataTableRow (Variables|Default|GetData%20Table) "37")
                                                (:then
                                                  (Default|UpdateDialogueTest (Variables|Default|GetdialogueWidget) (.IntroDialogue (Utilities|Struct|Breakdialogue_Structure _returnvalue_39)))
                                                  (Variables|Default|SetRow%20Name (.Row (Utilities|Struct|Breakdialogue_Structure _returnvalue_39)))
                                                  (Variables|Default|SetData%20Table (.Datatable (Utilities|Struct|Breakdialogue_Structure _returnvalue_39)))
                                                  ;[0.15 0.15 0.15 0.5] hide intro dialogue
                                                  (Variables|Default|Setenddialogue true)
                                                  (Utilities|FlowControl|Delay 5.0)
                                                  (Widget|SetVisibility (Variables|Default|GetdialogueWidget) "Hidden"))))))))))))))))))))))
        (:3
          (Development|PrintString "Dialogue Branch: Day 3 TRUTH Timeline")
          ;[0.15 0.15 0.15 0.5] dialoge line 38
          (bind _returnvalue_40 (Utilities|GetDataTableRow (Variables|Default|GetData%20Table) "38")
            (:then
              (bind _returnvalue_41 (UserInterface|CreateWidget "/Game/_Dialogue/UiTest.UiTest_C" 0 (Utilities|Text|ToText(Name) (Variables|Default|GetSpeakerName)) (.IntroDialogue (Utilities|Struct|Breakdialogue_Structure _returnvalue_40))))
              (bind _output_get_5 (Variables|Default|SetdialogueWidget _returnvalue_41))
              (UserInterface|Viewport|AddtoViewport _output_get_5 0)
              (Variables|Default|SetRow%20Name (.Row (Utilities|Struct|Breakdialogue_Structure _returnvalue_40)))
              (Variables|Default|SetData%20Table (.Datatable (Utilities|Struct|Breakdialogue_Structure _returnvalue_40)))
              (Variables|Default|Setenddialogue (.EndDialogue (Utilities|Struct|Breakdialogue_Structure _returnvalue_40)))
              (Utilities|FlowControl|Delay 5.0)
              ;[0.15 0.15 0.15 0.5] dialogue line 39
              (bind _returnvalue_42 (Utilities|GetDataTableRow (Variables|Default|GetData%20Table) "39")
                (:then
                  (Default|UpdateDialogueTest (Variables|Default|GetdialogueWidget) (.IntroDialogue (Utilities|Struct|Breakdialogue_Structure _returnvalue_42)))
                  (Variables|Default|SetRow%20Name (.Row (Utilities|Struct|Breakdialogue_Structure _returnvalue_42)))
                  (Variables|Default|SetData%20Table (.Datatable (Utilities|Struct|Breakdialogue_Structure _returnvalue_42)))
                  (Utilities|FlowControl|Delay 5.0)
                  ;[0.15 0.15 0.15 0.5] dialogue line 40
                  (bind _returnvalue_43 (Utilities|GetDataTableRow (Variables|Default|GetData%20Table) "40")
                    (:then
                      (Default|UpdateDialogueTest (Variables|Default|GetdialogueWidget) (.IntroDialogue (Utilities|Struct|Breakdialogue_Structure _returnvalue_43)))
                      (Variables|Default|SetRow%20Name (.Row (Utilities|Struct|Breakdialogue_Structure _returnvalue_43)))
                      (Variables|Default|SetData%20Table (.Datatable (Utilities|Struct|Breakdialogue_Structure _returnvalue_43)))
                      (Utilities|FlowControl|Delay 5.0)
                      ;[0.15 0.15 0.15 0.5] dialogue line 41
                      (bind _returnvalue_44 (Utilities|GetDataTableRow (Variables|Default|GetData%20Table) "41")
                        (:then
                          (Default|UpdateDialogueTest (Variables|Default|GetdialogueWidget) (.IntroDialogue (Utilities|Struct|Breakdialogue_Structure _returnvalue_44)))
                          (Variables|Default|SetRow%20Name (.Row (Utilities|Struct|Breakdialogue_Structure _returnvalue_44)))
                          (Variables|Default|SetData%20Table (.Datatable (Utilities|Struct|Breakdialogue_Structure _returnvalue_44)))
                          (Utilities|FlowControl|Delay 5.0)
                          ;[0.15 0.15 0.15 0.5] dialogue line 42
                          (bind _returnvalue_45 (Utilities|GetDataTableRow (Variables|Default|GetData%20Table) "42")
                            (:then
                              (Default|UpdateDialogueTest (Variables|Default|GetdialogueWidget) (.IntroDialogue (Utilities|Struct|Breakdialogue_Structure _returnvalue_45)))
                              (Variables|Default|SetRow%20Name (.Row (Utilities|Struct|Breakdialogue_Structure _returnvalue_45)))
                              (Variables|Default|SetData%20Table (.Datatable (Utilities|Struct|Breakdialogue_Structure _returnvalue_45)))
                              (Utilities|FlowControl|Delay 5.0)
                              ;[0.15 0.15 0.15 0.5] dialogue line 43
                              (bind _returnvalue_46 (Utilities|GetDataTableRow (Variables|Default|GetData%20Table) "43")
                                (:then
                                  (Default|UpdateDialogueTest (Variables|Default|GetdialogueWidget) (.IntroDialogue (Utilities|Struct|Breakdialogue_Structure _returnvalue_46)))
                                  (Variables|Default|SetRow%20Name (.Row (Utilities|Struct|Breakdialogue_Structure _returnvalue_46)))
                                  (Variables|Default|SetData%20Table (.Datatable (Utilities|Struct|Breakdialogue_Structure _returnvalue_46)))
                                  (Utilities|FlowControl|Delay 5.0)
                                  ;[0.15 0.15 0.15 0.5] dialogue line 44
                                  (bind _returnvalue_47 (Utilities|GetDataTableRow (Variables|Default|GetData%20Table) "44")
                                    (:then
                                      (Default|UpdateDialogueTest (Variables|Default|GetdialogueWidget) (.IntroDialogue (Utilities|Struct|Breakdialogue_Structure _returnvalue_47)))
                                      (Variables|Default|SetRow%20Name (.Row (Utilities|Struct|Breakdialogue_Structure _returnvalue_47)))
                                      (Variables|Default|SetData%20Table (.Datatable (Utilities|Struct|Breakdialogue_Structure _returnvalue_47)))
                                      (Utilities|FlowControl|Delay 5.0)
                                      ;[0.15 0.15 0.15 0.5] dialogue line 45
                                      (bind _returnvalue_48 (Utilities|GetDataTableRow (Variables|Default|GetData%20Table) "45")
                                        (:then
                                          (Default|UpdateDialogueTest (Variables|Default|GetdialogueWidget) (.IntroDialogue (Utilities|Struct|Breakdialogue_Structure _returnvalue_48)))
                                          (Variables|Default|SetRow%20Name (.Row (Utilities|Struct|Breakdialogue_Structure _returnvalue_48)))
                                          (Variables|Default|SetData%20Table (.Datatable (Utilities|Struct|Breakdialogue_Structure _returnvalue_48)))
                                          ;[0.15 0.15 0.15 0.5] hide intro dialogue
                                          (Variables|Default|Setenddialogue true)
                                          (Utilities|FlowControl|Delay 5.0)
                                          (Widget|SetVisibility (Variables|Default|GetdialogueWidget) "Hidden"))))))))))))))))))
        (:4
          (Development|PrintString "Dialogue Branch: Day 3 FALSE Timeline")
          ;[0.15 0.15 0.15 0.5] dialoge line 46
          (bind _returnvalue_49 (Utilities|GetDataTableRow (Variables|Default|GetData%20Table) "46")
            (:then
              (bind _returnvalue_50 (UserInterface|CreateWidget "/Game/_Dialogue/UiTest.UiTest_C" 0 (Utilities|Text|ToText(Name) (Variables|Default|GetSpeakerName)) (.IntroDialogue (Utilities|Struct|Breakdialogue_Structure _returnvalue_49))))
              (bind _output_get_6 (Variables|Default|SetdialogueWidget _returnvalue_50))
              (UserInterface|Viewport|AddtoViewport _output_get_6 0)
              (Variables|Default|SetRow%20Name (.Row (Utilities|Struct|Breakdialogue_Structure _returnvalue_49)))
              (Variables|Default|SetData%20Table (.Datatable (Utilities|Struct|Breakdialogue_Structure _returnvalue_49)))
              (Variables|Default|Setenddialogue (.EndDialogue (Utilities|Struct|Breakdialogue_Structure _returnvalue_49)))
              (Utilities|FlowControl|Delay 5.0)
              ;[0.15 0.15 0.15 0.5] dialogue line 47
              (bind _returnvalue_51 (Utilities|GetDataTableRow (Variables|Default|GetData%20Table) "47")
                (:then
                  (Default|UpdateDialogueTest (Variables|Default|GetdialogueWidget) (.IntroDialogue (Utilities|Struct|Breakdialogue_Structure _returnvalue_51)))
                  (Variables|Default|SetRow%20Name (.Row (Utilities|Struct|Breakdialogue_Structure _returnvalue_51)))
                  (Variables|Default|SetData%20Table (.Datatable (Utilities|Struct|Breakdialogue_Structure _returnvalue_51)))
                  (Utilities|FlowControl|Delay 5.0)
                  ;[0.15 0.15 0.15 0.5] dialogue line 48
                  (bind _returnvalue_52 (Utilities|GetDataTableRow (Variables|Default|GetData%20Table) "48")
                    (:then
                      (Default|UpdateDialogueTest (Variables|Default|GetdialogueWidget) (.IntroDialogue (Utilities|Struct|Breakdialogue_Structure _returnvalue_52)))
                      (Variables|Default|SetRow%20Name (.Row (Utilities|Struct|Breakdialogue_Structure _returnvalue_52)))
                      (Variables|Default|SetData%20Table (.Datatable (Utilities|Struct|Breakdialogue_Structure _returnvalue_52)))
                      (Utilities|FlowControl|Delay 5.0)
                      ;[0.15 0.15 0.15 0.5] dialogue line 49
                      (bind _returnvalue_53 (Utilities|GetDataTableRow (Variables|Default|GetData%20Table) "49")
                        (:then
                          (Default|UpdateDialogueTest (Variables|Default|GetdialogueWidget) (.IntroDialogue (Utilities|Struct|Breakdialogue_Structure _returnvalue_53)))
                          (Variables|Default|SetRow%20Name (.Row (Utilities|Struct|Breakdialogue_Structure _returnvalue_53)))
                          (Variables|Default|SetData%20Table (.Datatable (Utilities|Struct|Breakdialogue_Structure _returnvalue_53)))
                          (Utilities|FlowControl|Delay 5.0)
                          ;[0.15 0.15 0.15 0.5] dialogue line 50
                          (bind _returnvalue_54 (Utilities|GetDataTableRow (Variables|Default|GetData%20Table) "50")
                            (:then
                              (Default|UpdateDialogueTest (Variables|Default|GetdialogueWidget) (.IntroDialogue (Utilities|Struct|Breakdialogue_Structure _returnvalue_54)))
                              (Variables|Default|SetRow%20Name (.Row (Utilities|Struct|Breakdialogue_Structure _returnvalue_54)))
                              (Variables|Default|SetData%20Table (.Datatable (Utilities|Struct|Breakdialogue_Structure _returnvalue_54)))
                              (Utilities|FlowControl|Delay 5.0)
                              ;[0.15 0.15 0.15 0.5] dialogue line 51
                              (bind _returnvalue_55 (Utilities|GetDataTableRow (Variables|Default|GetData%20Table) "51")
                                (:then
                                  (Default|UpdateDialogueTest (Variables|Default|GetdialogueWidget) (.IntroDialogue (Utilities|Struct|Breakdialogue_Structure _returnvalue_55)))
                                  (Variables|Default|SetRow%20Name (.Row (Utilities|Struct|Breakdialogue_Structure _returnvalue_55)))
                                  (Variables|Default|SetData%20Table (.Datatable (Utilities|Struct|Breakdialogue_Structure _returnvalue_55)))
                                  (Utilities|FlowControl|Delay 5.0)
                                  ;[0.15 0.15 0.15 0.5] dialogue line 52
                                  (bind _returnvalue_56 (Utilities|GetDataTableRow (Variables|Default|GetData%20Table) "52")
                                    (:then
                                      (Default|UpdateDialogueTest (Variables|Default|GetdialogueWidget) (.IntroDialogue (Utilities|Struct|Breakdialogue_Structure _returnvalue_56)))
                                      (Variables|Default|SetRow%20Name (.Row (Utilities|Struct|Breakdialogue_Structure _returnvalue_56)))
                                      (Variables|Default|SetData%20Table (.Datatable (Utilities|Struct|Breakdialogue_Structure _returnvalue_56)))
                                      (Utilities|FlowControl|Delay 5.0)
                                      ;[0.15 0.15 0.15 0.5] dialogue line 53
                                      (bind _returnvalue_57 (Utilities|GetDataTableRow (Variables|Default|GetData%20Table) "53")
                                        (:then
                                          (Default|UpdateDialogueTest (Variables|Default|GetdialogueWidget) (.IntroDialogue (Utilities|Struct|Breakdialogue_Structure _returnvalue_57)))
                                          (Variables|Default|SetRow%20Name (.Row (Utilities|Struct|Breakdialogue_Structure _returnvalue_57)))
                                          (Variables|Default|SetData%20Table (.Datatable (Utilities|Struct|Breakdialogue_Structure _returnvalue_57)))
                                          (Utilities|FlowControl|Delay 5.0)
                                          ;[0.15 0.15 0.15 0.5] dialogue line 54
                                          (bind _returnvalue_58 (Utilities|GetDataTableRow (Variables|Default|GetData%20Table) "54")
                                            (:then
                                              (Default|UpdateDialogueTest (Variables|Default|GetdialogueWidget) (.IntroDialogue (Utilities|Struct|Breakdialogue_Structure _returnvalue_58)))
                                              (Variables|Default|SetRow%20Name (.Row (Utilities|Struct|Breakdialogue_Structure _returnvalue_58)))
                                              (Variables|Default|SetData%20Table (.Datatable (Utilities|Struct|Breakdialogue_Structure _returnvalue_58)))
                                              ;[0.15 0.15 0.15 0.5] hide intro dialogue
                                              (Variables|Default|Setenddialogue true)
                                              (Utilities|FlowControl|Delay 5.0)
                                              (Widget|SetVisibility (Variables|Default|GetdialogueWidget) "Hidden"))))))))))))))))))))
        (:5
          (goto _label))))
    (:CastFailed
      (Development|PrintString "cast failed, no dialogue will play"))))

(fn ConstructionScript)
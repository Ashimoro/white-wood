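; Intro dialogue Blueprint that automatically plays a timed twelve-line sequence when play begins, then hides it.
; BeginPlay creates a UiTest widget with the speaker name and first DataTable row, then pushes each later line through UpdateDialogueTest after a fixed delay.
; Lookups are a hardcoded nested chain: RowName picks only the first row, though each row rewrites it, and early rows can also swap the DataTable.
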(event EventBeginPlay
  ;[0.15 0.15 0.15 0.5] dialoge line 1
  (bind _returnvalue (Utilities|GetDataTableRow (Variables|Default|GetData%20Table) (Variables|Default|GetRow%20Name))
    (:then
      (bind _returnvalue_2 (UserInterface|CreateWidget "/Game/LevelPrototyping/UIButtonTest/UiTest.UiTest_C" 0 (Utilities|Text|ToText(Name) (Variables|Default|GetSpeakerName)) (.IntroDialogue (Utilities|Struct|Breakdialogue_Structure _returnvalue))))
      (bind _output_get (Variables|Default|SetdialogueWidget _returnvalue_2))
      (UserInterface|Viewport|AddtoViewport _output_get 0)
      (Variables|Default|SetRow%20Name (.Row (Utilities|Struct|Breakdialogue_Structure _returnvalue)))
      (Variables|Default|SetData%20Table (.Datatable (Utilities|Struct|Breakdialogue_Structure _returnvalue)))
      (Variables|Default|Setenddialogue (.EndDialogue (Utilities|Struct|Breakdialogue_Structure _returnvalue)))
      (Utilities|FlowControl|Delay 5.0)
      ;[0.15 0.15 0.15 0.5] dialogue line 2
      (bind _returnvalue_3 (Utilities|GetDataTableRow (Variables|Default|GetData%20Table) "2")
        (:then
          (Default|UpdateDialogueTest (Variables|Default|GetdialogueWidget) (.IntroDialogue (Utilities|Struct|Breakdialogue_Structure _returnvalue_3)))
          (Variables|Default|SetRow%20Name (.Row (Utilities|Struct|Breakdialogue_Structure _returnvalue_3)))
          (Variables|Default|SetData%20Table (.Datatable (Utilities|Struct|Breakdialogue_Structure _returnvalue_3)))
          (Utilities|FlowControl|Delay 5.0)
          ;[0.15 0.15 0.15 0.5] dialogue line 3
          (bind _returnvalue_4 (Utilities|GetDataTableRow (Variables|Default|GetData%20Table) "3")
            (:then
              (Default|UpdateDialogueTest (Variables|Default|GetdialogueWidget) (.IntroDialogue (Utilities|Struct|Breakdialogue_Structure _returnvalue_4)))
              (Variables|Default|SetRow%20Name (.Row (Utilities|Struct|Breakdialogue_Structure _returnvalue_4)))
              (Variables|Default|SetData%20Table (.Datatable (Utilities|Struct|Breakdialogue_Structure _returnvalue_4)))
              (Utilities|FlowControl|Delay 5.0)
              ;[0.15 0.15 0.15 0.5] dialogue line 4
              (bind _returnvalue_5 (Utilities|GetDataTableRow (Variables|Default|GetData%20Table) "4")
                (:then
                  (Default|UpdateDialogueTest (Variables|Default|GetdialogueWidget) (.IntroDialogue (Utilities|Struct|Breakdialogue_Structure _returnvalue_5)))
                  (Variables|Default|SetRow%20Name (.Row (Utilities|Struct|Breakdialogue_Structure _returnvalue_5)))
                  (Utilities|FlowControl|Delay 5.0)
                  ;[0.15 0.15 0.15 0.5] dialogue line 5
                  (bind _returnvalue_6 (Utilities|GetDataTableRow (Variables|Default|GetData%20Table) "5")
                    (:then
                      (Default|UpdateDialogueTest (Variables|Default|GetdialogueWidget) (.IntroDialogue (Utilities|Struct|Breakdialogue_Structure _returnvalue_6)))
                      (Variables|Default|SetRow%20Name (.Row (Utilities|Struct|Breakdialogue_Structure _returnvalue_6)))
                      (Utilities|FlowControl|Delay 5.0)
                      ;[0.15 0.15 0.15 0.5] dialogue line 6
                      (bind _returnvalue_7 (Utilities|GetDataTableRow (Variables|Default|GetData%20Table) "6")
                        (:then
                          (Default|UpdateDialogueTest (Variables|Default|GetdialogueWidget) (.IntroDialogue (Utilities|Struct|Breakdialogue_Structure _returnvalue_7)))
                          (Variables|Default|SetRow%20Name (.Row (Utilities|Struct|Breakdialogue_Structure _returnvalue_7)))
                          (Utilities|FlowControl|Delay 5.0)
                          ;[0.15 0.15 0.15 0.5] dialogue line 7
                          (bind _returnvalue_8 (Utilities|GetDataTableRow (Variables|Default|GetData%20Table) "7")
                            (:then
                              (Default|UpdateDialogueTest (Variables|Default|GetdialogueWidget) (.IntroDialogue (Utilities|Struct|Breakdialogue_Structure _returnvalue_8)))
                              (Variables|Default|SetRow%20Name (.Row (Utilities|Struct|Breakdialogue_Structure _returnvalue_8)))
                              (Utilities|FlowControl|Delay 5.0)
                              ;[0.15 0.15 0.15 0.5] dialogue line 8
                              (bind _returnvalue_9 (Utilities|GetDataTableRow (Variables|Default|GetData%20Table) "8")
                                (:then
                                  (Default|UpdateDialogueTest (Variables|Default|GetdialogueWidget) (.IntroDialogue (Utilities|Struct|Breakdialogue_Structure _returnvalue_9)))
                                  (Variables|Default|SetRow%20Name (.Row (Utilities|Struct|Breakdialogue_Structure _returnvalue_9)))
                                  (Utilities|FlowControl|Delay 5.0)
                                  ;[0.15 0.15 0.15 0.5] dialogue line 9
                                  (bind _returnvalue_10 (Utilities|GetDataTableRow (Variables|Default|GetData%20Table) "9")
                                    (:then
                                      (Default|UpdateDialogueTest (Variables|Default|GetdialogueWidget) (.IntroDialogue (Utilities|Struct|Breakdialogue_Structure _returnvalue_10)))
                                      (Variables|Default|SetRow%20Name (.Row (Utilities|Struct|Breakdialogue_Structure _returnvalue_10)))
                                      (Utilities|FlowControl|Delay 5.0)
                                      ;[0.15 0.15 0.15 0.5] dialogue line 10
                                      (bind _returnvalue_11 (Utilities|GetDataTableRow (Variables|Default|GetData%20Table) "10")
                                        (:then
                                          (Default|UpdateDialogueTest (Variables|Default|GetdialogueWidget) (.IntroDialogue (Utilities|Struct|Breakdialogue_Structure _returnvalue_11)))
                                          (Variables|Default|SetRow%20Name (.Row (Utilities|Struct|Breakdialogue_Structure _returnvalue_11)))
                                          (Utilities|FlowControl|Delay 5.0)
                                          ;[0.15 0.15 0.15 0.5] dialogue line 11
                                          (bind _returnvalue_12 (Utilities|GetDataTableRow (Variables|Default|GetData%20Table) "11")
                                            (:then
                                              (Default|UpdateDialogueTest (Variables|Default|GetdialogueWidget) (.IntroDialogue (Utilities|Struct|Breakdialogue_Structure _returnvalue_12)))
                                              (Variables|Default|SetRow%20Name (.Row (Utilities|Struct|Breakdialogue_Structure _returnvalue_12)))
                                              (Utilities|FlowControl|Delay 5.0)
                                              ;[0.15 0.15 0.15 0.5] dialogue line 12
                                              (bind _returnvalue_13 (Utilities|GetDataTableRow (Variables|Default|GetData%20Table) "12")
                                                (:then
                                                  (Default|UpdateDialogueTest (Variables|Default|GetdialogueWidget) (.IntroDialogue (Utilities|Struct|Breakdialogue_Structure _returnvalue_13)))
                                                  (Variables|Default|SetRow%20Name (.Row (Utilities|Struct|Breakdialogue_Structure _returnvalue_13)))
                                                  ;[0.15 0.15 0.15 0.5] hide intro dialogue
                                                  (Variables|Default|Setenddialogue true)
                                                  (Utilities|FlowControl|Delay 5.0)
                                                  (Widget|SetVisibility (Variables|Default|GetdialogueWidget) "Hidden"))))))))))))))))))))))))))

(fn ConstructionScript)
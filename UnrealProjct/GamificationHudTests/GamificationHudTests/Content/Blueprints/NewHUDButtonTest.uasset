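; Test actor that plays a three-line intro dialogue on screen from data table rows when play begins.
; It creates a dialogue widget with the speaker name and first line, updates it at fixed delays, then hides it.
; Each row supplies the next table, but the second and third row names are hardcoded rather than using the stored row link.
; The end-dialogue flag is set but never read here.
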(event EventBeginPlay
  ;[0.15 0.15 0.15 0.5] dialoge line 1
  (bind _returnvalue (Utilities|GetDataTableRow (Variables|Default|GetData%20Table) (Variables|Default|GetRow%20Name))
    (:then
      (bind _returnvalue_2 (UserInterface|CreateWidget "/Game/LevelPrototyping/UIButtonTest/UiTest.UiTest_C" 0 (Utilities|Text|ToText(Name) (Variables|Default|GetSpeakerName)) (.IntroDialogue (Utilities|Struct|Breakdialogue_Structure _returnvalue))))
      (bind _output_get (Variables|Default|SetdialogueWidget _returnvalue_2))
      (UserInterface|Viewport|AddtoViewport _output_get 0)
      (Variables|Default|SetRow%20Name (.Row (Utilities|Struct|Breakdialogue_Structure _returnvalue)))
      (Variables|Default|SetData%20Table (.Datatable (Utilities|Struct|Breakdialogue_Structure _returnvalue)))
      (Variables|Default|Setenddialogue (.EndDialogue (Utilities|Struct|Breakdialogue_Structure _returnvalue)))
      (Utilities|FlowControl|Delay 2.0)
      ;[0.15 0.15 0.15 0.5] dialogue line 2
      (bind _returnvalue_3 (Utilities|GetDataTableRow (Variables|Default|GetData%20Table) "2")
        (:then
          (Default|UpdateDialogueTest (Variables|Default|GetdialogueWidget) (.IntroDialogue (Utilities|Struct|Breakdialogue_Structure _returnvalue_3)))
          (Variables|Default|SetRow%20Name (.Row (Utilities|Struct|Breakdialogue_Structure _returnvalue_3)))
          (Variables|Default|SetData%20Table (.Datatable (Utilities|Struct|Breakdialogue_Structure _returnvalue_3)))
          (Utilities|FlowControl|Delay 2.0)
          ;[0.15 0.15 0.15 0.5] dialogue line 3
          (bind _returnvalue_4 (Utilities|GetDataTableRow (Variables|Default|GetData%20Table) "3")
            (:then
              (Default|UpdateDialogueTest (Variables|Default|GetdialogueWidget) (.IntroDialogue (Utilities|Struct|Breakdialogue_Structure _returnvalue_4)))
              (Variables|Default|SetRow%20Name (.Row (Utilities|Struct|Breakdialogue_Structure _returnvalue_4)))
              (Variables|Default|SetData%20Table (.Datatable (Utilities|Struct|Breakdialogue_Structure _returnvalue_4)))
              (Variables|Default|Setenddialogue true)
              (Utilities|FlowControl|Delay 2.0)
              (Widget|SetVisibility (Variables|Default|GetdialogueWidget) "Hidden"))))))))

(fn ConstructionScript)